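; BP_porte is a locked door that opens only for a third-person character holding its key.
; Entering the box trigger enables the door's input if the character's KeyListe boolean at index DoorID is true.
; Pressing E then plays the Ouverture timeline, which rotates the mesh through MakeRotFromZ.
; Leaving the trigger disables input and reverses the timeline to close the door.
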(event OnComponentBeginOverlap(Box)
  (params (OverlappedComponent :type Primitive%20Component%20Object%20Reference) (OtherActor :type Actor%20Object%20Reference) (OtherComp :type Primitive%20Component%20Object%20Reference) (OtherBodyIndex :type Integer) (bFromSweep :type Boolean) (SweepResult :type Hit%20Result%20Structure%20%28by%20ref%29))
  (bind _asbp_third_person_character (Utilities|Casting|CastToBP_ThirdPersonCharacter OtherActor))
  (for (_array_element _array_index) (Variables|/Game/ThirdPerson/Blueprints/BP_ThirdPersonCharacter.BP_ThirdPersonCharacter_C|Getkey_liste _asbp_third_person_character)
    (if (and (== _array_index (Variables|Default|GetDoorID)) _array_element)
      (Input|EnableInput (Game|GetPlayerController 0)))))

(event OnComponentEndOverlap(Box)
  (params (OverlappedComponent :type Primitive%20Component%20Object%20Reference) (OtherActor :type Actor%20Object%20Reference) (OtherComp :type Primitive%20Component%20Object%20Reference) (OtherBodyIndex :type Integer))
  (Utilities|Casting|CastToBP_ThirdPersonCharacter OtherActor)
  (Input|DisableInput (Game|GetPlayerController 0))
  (bind _ouverture_porte (Timeline|Ouverture Reverse)
    (:Update
      (Transformation|SetRelativeRotation (Variables|Default|GetStaticMesh) (Math|Rotator|MakeRotfromZ _ouverture_porte) false false))))

(event Input|KeyboardEvents|E
  (params (Key :type Key%20Structure :default "None"))
  (:Pressed
    (bind _ouverture_porte (Timeline|Ouverture Play)
      (:Update
        (Transformation|SetRelativeRotation (Variables|Default|GetStaticMesh) (Math|Rotator|MakeRotfromZ _ouverture_porte) false false)))))

(fn ConstructionScript)